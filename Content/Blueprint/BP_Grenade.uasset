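; BP_Grenade is a grenade pickup that spins in place until a BP_Player overlaps its sphere.
; Tick adds a constant world rotation to the grenade component.
; On overlap it increments the player's grenade count, sets its grenade flag, and destroys itself.
; It also unhides the player's own Grenade component and snaps it to the right thigh socket on the mesh.
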(event OnComponentBeginOverlap(Sphere)
  (params (OverlappedComponent :type Primitive%20Component%20Object%20Reference) (OtherActor :type Actor%20Object%20Reference) (OtherComp :type Primitive%20Component%20Object%20Reference) (OtherBodyIndex :type Integer) (bFromSweep :type Boolean) (SweepResult :type Hit%20Result%20Structure%20%28by%20ref%29))
  (bind _asbp_player (Utilities|Casting|CastToBP_Player OtherActor))
  (Variables|/Game/Blueprint/BP_Player.BP_Player_C|SetGCount _asbp_player (+ (Variables|/Game/Blueprint/BP_Player.BP_Player_C|GetGCount _asbp_player) 1))
  (Actor|DestroyActor)
  (Variables|/Game/Blueprint/BP_Player.BP_Player_C|SetHaveGrenade? _asbp_player true)
  (Development|SetHiddeninGame (Variables|/Game/Blueprint/BP_Player.BP_Player_C|GetGrenade _asbp_player) false false)
  (Transformation|AttachComponentToComponent (Variables|/Game/Blueprint/BP_Player.BP_Player_C|GetGrenade _asbp_player) (Variables|/Script/Engine.Character|GetMesh _asbp_player) "thigh_rSocket" "SnapToTarget" "SnapToTarget" "SnapToTarget" true))

(event EventTick
  (params (DeltaSeconds :type Float%20%28single-precision%29))
  (Transformation|AddWorldRotation (Variables|Default|GetGrenade) "0.000000,1.000000,0.000000" false false))

(fn ConstructionScript)